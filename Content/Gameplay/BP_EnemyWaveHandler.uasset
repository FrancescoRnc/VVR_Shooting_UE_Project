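; BP_EnemyWaveHandler sequences enemy waves in the VR shooter from an indexed list of wave info.
; On BeginPlay it registers itself in GI_VRShooter, the game instance.
; StartWaving makes the wave at the current index and prints the remaining count.
; OnWaveEmpty advances the index and calls CallPlayAfterEmptyWave only while waves remain, with no handling here for the end of the list.
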(event EventBeginPlay
  (Variables|/Game/GI_VRShooter.GI_VRShooter_C|SetWaveHandlerRef (.AsGI%20VRShooter (Utilities|Casting|CastToGI_VRShooter (Game|GetGameInstance))) self))

(event EventStartWaving
  (Class|EnemyWaveHandler|MakeWave (Utilities|Array|Get(acopy) (Variables|Default|GetWaveInfoList) (Variables|Default|GetCurrentWaveIndex)))
  (Development|PrintString (Utilities|String|Append "Remaining: " (Utilities|String|ToString(Integer) (Variables|Default|GetCurrentWaveCount)))))

(event EventOnWaveEmpty
  (bind _currentwaveindex (Variables|Default|GetCurrentWaveIndex))
  (Math|Integer|IncrementInt _currentwaveindex
    (:%20%20
      (if (< _currentwaveindex (Utilities|Array|Length (Variables|Default|GetWaveInfoList)))
        (Default|CallPlayAfterEmptyWave)))))

(fn ConstructionScript)