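; BP_EnemyBall is a floating ball enemy with health that is reused through despawn and respawn.
; Despawn disables collision, stops movement, fades out and relocates the ball below, while Respawn restores health and collision, restarts movement and fades in.
; An UpDown timeline drives a frame-rate-scaled vertical bob.
; GetDamage subtracts health and returns whether it is depleted, and Die reports to the owning EnemyManager's WaveGenerator.
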(event Custom|Opacity%20Effect
  (params (Value :type Float%20%28single-precision%29))
  (Rendering|Material|SetScalarParameterValue (Variables|Default|GetMaterial) "Opacity" Value :!class /Script/Engine.MaterialInstanceDynamic))

(event EventRespawn
  (Class|EnemyBall|RestoreHealth)
  (Collision|SetCollisionEnabled (Variables|Default|GetCollision) "QueryAndPhysics")
  (Class|CmpUpDownInterface|Move)
  (bind _value (Timeline|Respawn%20Fade PlayFromStart)
    (:Update
      (CallFunction|OpacityEffect _value))))

(event EventDeSpawn
  (Collision|SetCollisionEnabled (Variables|Default|GetCollision) "NoCollision")
  (Class|CmpUpDownInterface|Stop)
  (bind _value (Timeline|Despawn%20Fade PlayFromStart)
    (:Update
      (CallFunction|OpacityEffect _value))
    (:Finished
      (Class|EnemyBall|Locate (Math|Vector|MakeVector 0.0 0.0 -5e+02)))))

(event EventDie
  (Class|EnemyWaveGenerator|UpdateCurrentWaveStats (Variables|/Script/VR_Shooting.EnemyManager|GetWaveGenerator (.AsEnemy%20Manager (Utilities|Casting|CastToEnemyManager (Utilities|GetOuterObject (Variables|Default|GetManagerOwner))))) self))

(event EventBeginPlay)

(event EventMove
  (bind _value_nrm (Timeline|UpDown PlayFromStart)
    (:Update
      (Transformation|AddActorLocalOffset (Math|Vector|MakeVector 0.0 0.0 (* (* _value_nrm 2.5e+02) (Utilities|Time|GetWorldDeltaSeconds))) false false))))

(event EventStop
  (bind _value_nrm (Timeline|UpDown Stop)
    (:Update
      (Transformation|AddActorLocalOffset (Math|Vector|MakeVector 0.0 0.0 (* (* _value_nrm 2.5e+02) (Utilities|Time|GetWorldDeltaSeconds))) false false))))

(fn ConstructionScript)

(fn GetDamage
  (params (amount :type Float%20%28single-precision%29))
  (bind _output_get (Variables|Default|SetCurHealthValue (- (Variables|Default|GetCurHealthValue) amount)))
  (return (<= _output_get 0.0)))

(fn GetHealthValue
  (return (Variables|Default|GetCurHealthValue)))