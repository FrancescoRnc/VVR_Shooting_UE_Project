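; Base pooled bullet actor for the VR shooter, reused through a queue in GI_VRShooter rather than destroyed.
; SpawnonShoot places and enables it; Tick moves it forward without sweeping and counts down a custom lifespan.
; When the lifespan expires, it re-enqueues itself and resets the timer.
; Overlaps send damage and possibly death messages, then disable visibility, collision and tick without re-enqueuing.
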(event OnComponentBeginOverlap(Collision)
  (params (OverlappedComponent :type Primitive%20Component%20Object%20Reference) (OtherActor :type Actor%20Object%20Reference) (OtherComp :type Primitive%20Component%20Object%20Reference) (OtherBodyIndex :type Integer) (bFromSweep :type Boolean) (SweepResult :type Hit%20Result%20Structure%20%28by%20ref%29))
  (Development|PrintString (Utilities|String|Append "Collided with " (Utilities|GetDisplayName OtherActor)))
  (bind _returnvalue (Class|DamageableInterface|GetDamage(Message) OtherActor (Variables|Default|GetDamageValue)))
  (if _returnvalue
    (Class|DamageableInterface|Die(Message) OtherActor))
  (Class|GunBullet|SetNewAvailability false))

(event EventSpawnonShoot
  (params (startLoc :type Vector%20%28by%20ref%29 :default "0, 0, 0") (startRot :type Rotator%20%28by%20ref%29 :default "0, 0, 0"))
  (Transformation|SetActorLocationAndRotation startLoc startRot)
  (Class|GunBullet|SetNewAvailability true)
  (Utilities|FlowControl|DoOnce false) ; enters at Reset
)

(event EventTick
  (params (DeltaSeconds :type Float%20%28single-precision%29))
  (bind _output_get (Variables|Default|SetCustomLifeSpan (- (Variables|Default|GetCustomLifeSpan) DeltaSeconds)))
  (Transformation|AddActorWorldOffset (* (Transformation|GetActorForwardVector) (* (Variables|Default|GetSpeed) DeltaSeconds)))
  (if (<= _output_get 0.0)
    (Utilities|FlowControl|DoOnce false
      (:Completed
        (Class|BulletInterface|OnEndLifespan)))))

(event EventSetNewAvailability
  (params (value :type Boolean))
  (Rendering|SetVisibility (Variables|Default|GetStaticMesh) value true)
  (Collision|SetCollisionEnabled (Variables|Default|GetCollision) (select value "QueryAndPhysics" "NoCollision"))
  (Actor|Tick|SetActorTickEnabled value))

(event EventRegenerate
  (Variables|Default|SetCustomLifeSpan (Variables|Default|GetMaxCustomLifeSpan)))

(event EventOnEndLifespan
  (Default|EnqueueBulletinQueue (.AsGI%20VRShooter (Utilities|Casting|CastToGI_VRShooter (Game|GetGameInstance))) self)
  (Class|BulletInterface|Regenerate))

(fn ConstructionScript)